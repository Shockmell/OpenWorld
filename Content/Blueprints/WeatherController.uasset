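; Weather controller actor that runs a scripted sequence from clouding and gloom through a rainy spell and back.
; BeginPlay snaps the rain particles to the player, then uses timed delays to set targets and toggle rain particles and audio.
; Each Tick, three macros step sky cloud opacity and the MP_Global Gloom and RainLevel parameters toward those targets by a shared signed ChangeRate, then refresh the sky.
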(event Custom|ToggleRain
  (params (Enable :type Boolean))
  (if Enable
    (Components|Activation|SetActive (Variables|Default|GetP_Rain) true false)
    (Audio|Components|Audio|Play (Variables|Default|Getrain-03) 0.0)
    (Variables|Default|SetchangeRate 0.1)
    (Variables|Default|SettargetRainLevel 0.9)
    (else
      (Components|Activation|SetActive (Variables|Default|GetP_Rain) false false)
      (Variables|Default|SetchangeRate -0.1)
      (Variables|Default|SettargetRainLevel 0.1)
      (Utilities|FlowControl|Delay 4.0)
      (Audio|Components|Audio|Stop (Variables|Default|Getrain-03)))))

(event EventBeginPlay
  (Utilities|FlowControl|Delay 0.2)
  (Transformation|AttachComponentToComponent (Variables|Default|GetP_Rain) (Variables|/Script/Engine.Actor|GetRootComponent (Game|GetPlayerCharacter 0)) "None" "SnapToTarget" "SnapToTarget" "SnapToTarget" true)
  (Utilities|FlowControl|Delay 5.0)
  (Variables|Default|SettargetCloudOpacity 5.0)
  (Variables|Default|SettargetGloom 0.05)
  (Utilities|FlowControl|Delay 2e+01)
  (CallFunction|ToggleRain true)
  (Utilities|FlowControl|Delay 3e+01)
  (CallFunction|ToggleRain false)
  (Variables|Default|SettargetCloudOpacity 0.7)
  (Variables|Default|SettargetGloom 1.0))

(event Collision|EventActorBeginOverlap
  (params (OtherActor :type Actor%20Object%20Reference)))

(event EventTick
  (params (DeltaSeconds :type Float%20%28single-precision%29))
  (|UpdateSkyColor
    (:OutputPin
      (|UpdateSky
        (:OutputPin
          (|Raining
            (:OutputPin
              (Default|UpdateSky (Variables|Default|GetSky)))))))))

(fn ConstructionScript)